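; Player character Blueprint, named for the player menu, that plays dance emotes on its mesh.
; BeginPlay adds the IMC_Game mapping context to the controlling player's Enhanced Input subsystem.
; IA_Emote plays Gangnam_Style and a hardcoded 2 key plays Dancing_Twerk, both unlooped.
; After a fixed delay, each re-sets the mesh to single-node animation mode rather than returning it to an Animation Blueprint.
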(event Input|EnhancedActionEvents|EnhancedInputActionIA_Emote
  (params (ActionValue :type Boolean) (ElapsedSeconds :type Float%20%28double-precision%29) (TriggeredSeconds :type Float%20%28double-precision%29) (InputAction :type Input%20Action%20Object%20Reference :default "/Game/TopDown/Input/Actions/IA_Emote.IA_Emote"))
  (Components|Animation|PlayAnimation (Variables|Character|GetMesh) "/Game/Characters/GameChar/Animations/Emote/Gangnam_Style.Gangnam_Style" false)
  (Utilities|FlowControl|Delay 13.0)
  (Components|Animation|SetAnimationMode (Variables|Character|GetMesh) "AnimationSingleNode" true))

(event EventBeginPlay
  (bind _asplayer_controller (Utilities|Casting|CastToPlayerController (Pawn|GetController)))
  (Utilities|IsValid (PlayerController|LocalPlayerSubsystems|GetEnhancedInputLocalPlayerSubsystem _asplayer_controller)
    (:Is%20Valid
      (Input|AddMappingContext (PlayerController|LocalPlayerSubsystems|GetEnhancedInputLocalPlayerSubsystem _asplayer_controller) "/Game/TopDown/Input/IMC_Game.IMC_Game" 0 "(bIgnoreAllPressedKeysUntilRelease=True,bForceImmediately=False,bNotifyUserSettings=False)"))))

(event Input|KeyboardEvents|2
  (params (Key :type Key%20Structure :default "None"))
  (:Pressed
    (Components|Animation|PlayAnimation (Variables|Character|GetMesh) "/Game/Characters/GameChar/Animations/Emote/Dancing_Twerk.Dancing_Twerk" false)
    (Utilities|FlowControl|Delay 12.0)
    (Components|Animation|SetAnimationMode (Variables|Character|GetMesh) "AnimationSingleNode" true)))

(fn ConstructionScript)