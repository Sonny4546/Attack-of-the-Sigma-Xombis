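; Player character for a top-down shooter with world-axis movement, cursor-facing rotation, mouse-wheel zoom, a cooldown dive roll and dance emotes.
; Firing spawns BP_Bullet and spends ammo, reloading draws from a reserve, and damage lowers health until PlayerDead disables input, movement and collision.
; Dispatchers broadcast health and ammo every Tick, plus reload, no-ammo and death events.
; One-off animations override the mesh, usually restoring the Animation Blueprint after fixed delays.
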(event Input|EnhancedActionEvents|EnhancedInputActionIA_Gun
  (params (ActionValue :type Boolean) (ElapsedSeconds :type Float%20%28double-precision%29) (TriggeredSeconds :type Float%20%28double-precision%29) (InputAction :type Input%20Action%20Object%20Reference :default "/Game/TopDown/Input/Actions/IA_Gun.IA_Gun"))
  (if (<= (Variables|Default|GetAmmo) 0)
    (Default|CallReload)
    (else
      (Audio|PlaySoundatLocation "/Game/Audio/gunshot.gunshot" (Transformation|GetWorldLocation (Variables|Default|GetBP_Gun)) "0, 0, 0" 1.0 1.0 0.0 0 0 0 0)
      (Variables|Default|SetAmmo (- (Variables|Default|GetAmmo) 1))
      (Game|SpawnActorfromClass "/Game/Characters/GameChar/Weapons/BP_Bullet.BP_Bullet_C" (Math|Transform|MakeTransform (Transformation|GetWorldLocation (Variables|Default|GetBulletSpawn)) (Transformation|GetActorRotation (Components|GetOwner (Variables|Character|GetMesh)))) "AlwaysSpawn" "MultiplyWithRoot" 0 0)
      (if (> (Math|Vector|VectorLength (Pawn|Components|CharacterMovement|GetCurrentAcceleration (Variables|Character|GetCharacterMovement))) 0.0)
        _
        (else
          (Components|Animation|PlayAnimation (Variables|Character|GetMesh) "/Game/Characters/GameChar/Animations/DukeDennis/firing_rifle.firing_rifle" false)))
      (Utilities|FlowControl|Delay 0.75)
      (Components|Animation|SetAnimationMode (Variables|Character|GetMesh) "AnimationBlueprint" true)
      (if (<= (Variables|Default|GetPlayerHP) 0.0)
        (CallFunction|PlayerDead)))))

(event Input|EnhancedActionEvents|EnhancedInputActionIA_WASDControl
  (params (ActionValue :type Vector%202D%20Structure) (ElapsedSeconds :type Float%20%28double-precision%29) (TriggeredSeconds :type Float%20%28double-precision%29) (InputAction :type Input%20Action%20Object%20Reference :default "/Game/TopDown/Input/Actions/IA_WASDControl.IA_WASDControl"))
  (:Triggered
    (Pawn|Input|AddMovementInput "0.000000,1.000000,0.000000" (.x ActionValue) false)
    (Pawn|Input|AddMovementInput "1.000000,0.000000,0.000000" (.y ActionValue) false)))

(event Input|EnhancedActionEvents|EnhancedInputActionIA_Mouse
  (params (ActionValue :type Vector%202D%20Structure) (ElapsedSeconds :type Float%20%28double-precision%29) (TriggeredSeconds :type Float%20%28double-precision%29) (InputAction :type Input%20Action%20Object%20Reference :default "/Game/TopDown/Input/Actions/IA_Mouse.IA_Mouse"))
  (bind _returnvalue (Transformation|GetActorRotation))
  (Transformation|SetActorRotation (Math|Rotator|MakeRotator (.roll _returnvalue) (.pitch _returnvalue) (.yaw (Math|Interpolation|RInterpTo (Transformation|GetActorRotation) (Math|Rotator|FindLookatRotation (+ "" "") (- (.ImpactPoint (Collision|BreakHitResult (.HitResult (Game|Player|GetHitResultUnderCursorbyChannel (Game|GetPlayerController 0) "TraceTypeQuery1" true)))) (Transformation|GetActorLocation))) (Utilities|Time|GetWorldDeltaSeconds) (Variables|Default|GetInterp%20Speed))))))

(event Input|EnhancedActionEvents|EnhancedInputActionIA_Emote
  (params (ActionValue :type Boolean) (ElapsedSeconds :type Float%20%28double-precision%29) (TriggeredSeconds :type Float%20%28double-precision%29) (InputAction :type Input%20Action%20Object%20Reference :default "/Game/TopDown/Input/Actions/IA_Emote.IA_Emote"))
  (Components|Animation|PlayAnimation (Variables|Character|GetMesh) "/Game/Characters/GameChar/Animations/Emote/Gangnam_Style.Gangnam_Style" false)
  (Utilities|FlowControl|Delay 13.0)
  (Components|Animation|SetAnimationMode (Variables|Character|GetMesh) "AnimationBlueprint" true))

(event Game|Damage|EventAnyDamage
  (params (Damage :type Float%20%28single-precision%29) (DamageType :type Damage%20Type%20Object%20Reference) (InstigatedBy :type Controller%20Object%20Reference) (DamageCauser :type Actor%20Object%20Reference))
  (bind _output_get (Variables|Default|SetDamage Damage))
  (bind _output_get_2 (Variables|Default|SetPlayerHP (- (Variables|Default|GetPlayerHP) _output_get)))
  (if (<= _output_get_2 0.0)
    (Development|PrintString "DEAD!")
    (CallFunction|PlayerDead)
    (else
      (Development|PrintString "OUCH")
      (Components|Animation|PlayAnimation (Variables|Character|GetMesh) "/Game/Characters/GameChar/Animations/DukeDennis/hit_reaction.hit_reaction" false)
      (Utilities|FlowControl|Delay 0.2)
      (Components|Animation|SetAnimationMode (Variables|Character|GetMesh) "AnimationBlueprint" true))))

(event EventBeginPlay
  (bind _asplayer_controller (Utilities|Casting|CastToPlayerController (Pawn|GetController)))
  (Utilities|IsValid (PlayerController|LocalPlayerSubsystems|GetEnhancedInputLocalPlayerSubsystem _asplayer_controller)
    (:Is%20Valid
      (Input|AddMappingContext (PlayerController|LocalPlayerSubsystems|GetEnhancedInputLocalPlayerSubsystem _asplayer_controller) "/Game/TopDown/Input/IMC_Game.IMC_Game" 0 "(bIgnoreAllPressedKeysUntilRelease=True,bForceImmediately=False,bNotifyUserSettings=False)"))))

(event EventTick
  (params (DeltaSeconds :type Float%20%28single-precision%29))
  (Default|CallPlayerHealth (Variables|Default|GetPlayerHP))
  (Default|CallPlayerAmmo (Variables|Default|GetAmmo) (Variables|Default|GetMaxAmmo)))

(event Input|KeyboardEvents|2
  (params (Key :type Key%20Structure :default "None"))
  (:Pressed
    (Components|Animation|PlayAnimation (Variables|Character|GetMesh) "/Game/Characters/GameChar/Animations/Emote/Dancing_Twerk.Dancing_Twerk" false)
    (Utilities|FlowControl|Delay 12.0)
    (Components|Animation|SetAnimationMode (Variables|Character|GetMesh) "AnimationBlueprint" true)))

(event Input|KeyboardEvents|Q
  (params (Key :type Key%20Structure :default "None"))
  (bind _mesh (Variables|Character|GetMesh))
  (:Pressed
    (if (Variables|Default|GetSlide)
      (Variables|/Script/Engine.CharacterMovementComponent|SetMaxWalkSpeed (Variables|Character|GetCharacterMovement) 1e+03)
      (Components|Animation|PlayAnimation _mesh "/Game/Characters/GameChar/Animations/DukeDennis/Running_Dive_Roll.Running_Dive_Roll" false)
      (Utilities|FlowControl|Delay 1.0)
      (Components|Animation|SetAnimationMode _mesh "AnimationBlueprint" true)
      (Variables|/Script/Engine.CharacterMovementComponent|SetMaxWalkSpeed (Variables|Character|GetCharacterMovement) 6e+02)
      (Variables|Default|SetSlide false)
      (Utilities|FlowControl|Delay 2.0)
      (Variables|Default|SetSlide true))))

(event Input|MouseEvents|MouseWheelUp
  (params (Key :type Key%20Structure :default "None"))
  (:Pressed
    (Variables|/Script/Engine.SpringArmComponent|SetTargetArmLength (Variables|Camera|GetSpringArm) (Math|Float|Clamp(Float) (- (Variables|/Script/Engine.SpringArmComponent|GetTargetArmLength (Variables|Camera|GetSpringArm)) 1e+02) 5e+02 8e+03))))

(event Input|MouseEvents|MouseWheelDown
  (params (Key :type Key%20Structure :default "None"))
  (:Pressed
    (Variables|/Script/Engine.SpringArmComponent|SetTargetArmLength (Variables|Camera|GetSpringArm) (Math|Float|Clamp(Float) (+ (Variables|/Script/Engine.SpringArmComponent|GetTargetArmLength (Variables|Camera|GetSpringArm)) 1e+02) 1e+02 8e+03))))

(event Input|KeyboardEvents|R
  (params (Key :type Key%20Structure :default "None"))
  (:Pressed
    (if (not (Variables|Default|GetReloadAgainDelay))
      (Variables|Default|SetReloadAgainDelay true)
      (if (<= (Variables|Default|GetMaxAmmo) 0)
        (Default|CallNoAmmo)
        (Variables|Default|SetReloadAgainDelay false)
        (elif (<= (Variables|Default|GetMaxAmmo) 50)
          (Variables|Default|SetMaxAmmo (- (Variables|Default|GetMaxAmmo) 50))
          (Variables|Default|SetAmmo (+ (Variables|Default|GetAmmo) 50))
          (Utilities|FlowControl|Delay 1.0)
          (Variables|Default|SetReloadAgainDelay false)
          (else
            (Variables|Default|SetMaxAmmo (- (Variables|Default|GetMaxAmmo) 100))
            (Variables|Default|SetAmmo (+ (Variables|Default|GetAmmo) 100))
            (Utilities|FlowControl|Delay 2.0)
            (Variables|Default|SetReloadAgainDelay false)))))))

(fn ConstructionScript)

(fn PlayerDead
  (Components|Animation|PlayAnimation (Variables|Character|GetMesh) "/Game/Characters/GameChar/Animations/DukeDennis/walking_to_dying.walking_to_dying" false)
  (Pawn|Components|CharacterMovement|DisableMovement (Variables|Character|GetCharacterMovement))
  (Input|DisableInput (Game|GetPlayerController 0))
  (Collision|SetCollisionEnabled (Variables|Collision|GetCapsuleComponent) "NoCollision")
  (Default|CallDead))