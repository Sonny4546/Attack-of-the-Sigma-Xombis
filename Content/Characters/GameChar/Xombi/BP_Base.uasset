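; BP_Base is a zombie character base Blueprint that provides shared death and hit-reaction functions.
; Both functions halt and disable CharacterMovement, set the mode to Walking, then play a one-shot animation directly on the Mesh.
; ZombieDead also turns off collision on the body and extra colliders, sets a short lifespan and calls ZombieKilled.
; ZombieHit returns the Mesh and contains no logic to restart movement.
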(fn ConstructionScript)

(fn ZombieDead
  (bind _charactermovement (Variables|Character|GetCharacterMovement))
  (Pawn|Components|CharacterMovement|DisableMovement _charactermovement)
  (Class|NavMovementComponent|StopActiveMovement _charactermovement)
  (Components|Movement|StopMovementImmediately _charactermovement)
  (Pawn|Components|CharacterMovement|SetMovementMode _charactermovement "MOVE_Walking" 0)
  (Components|Animation|PlayAnimation (Variables|Character|GetMesh) "/Game/Characters/GameChar/Animations/Xombie/Zombie_Death.Zombie_Death" false)
  (Actor|SetLifeSpan 4.0)
  (Collision|SetCollisionEnabled (Variables|Default|GetLeft) "NoCollision")
  (Default|CallZombieKilled))

(fn ZombieHit
  (bind _charactermovement (Variables|Character|GetCharacterMovement))
  (bind _mesh (Variables|Character|GetMesh))
  (Pawn|Components|CharacterMovement|DisableMovement _charactermovement)
  (Class|NavMovementComponent|StopActiveMovement _charactermovement)
  (Components|Movement|StopMovementImmediately _charactermovement)
  (Pawn|Components|CharacterMovement|SetMovementMode _charactermovement "MOVE_Walking" 0)
  (Components|Animation|PlayAnimation _mesh "/Game/Characters/GameChar/Animations/Xombie/zombie_reaction_hit.zombie_reaction_hit" false)
  (return _mesh))