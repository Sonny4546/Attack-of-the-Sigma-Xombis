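; Main zombie enemy character that materializes on spawn, hunts the player and dissolves on death.
; After the reversed dissolve timeline on BeginPlay, an AI MoveTo loop chases the player, plays an attack animation, then repeats while alive.
; Left and Right component overlaps deal damage to BP_Player.
; Incoming damage lowers health, triggering a hit reaction and renewed chase, or death with dynamic-material dissolve.
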(event OnComponentBeginOverlap(Right)
  (params (OverlappedComponent :type Primitive%20Component%20Object%20Reference) (OtherActor :type Actor%20Object%20Reference) (OtherComp :type Primitive%20Component%20Object%20Reference) (OtherBodyIndex :type Integer) (bFromSweep :type Boolean) (SweepResult :type Hit%20Result%20Structure%20%28by%20ref%29))
  (bind _asbp_player (Utilities|Casting|CastToBP_Player OtherActor))
  (bind _returnvalue (Game|Damage|ApplyDamage _asbp_player 2.0 0 self)))

(event OnComponentBeginOverlap(Left)
  (params (OverlappedComponent :type Primitive%20Component%20Object%20Reference) (OtherActor :type Actor%20Object%20Reference) (OtherComp :type Primitive%20Component%20Object%20Reference) (OtherBodyIndex :type Integer) (bFromSweep :type Boolean) (SweepResult :type Hit%20Result%20Structure%20%28by%20ref%29))
  (bind _asbp_player (Utilities|Casting|CastToBP_Player OtherActor))
  (bind _returnvalue (Game|Damage|ApplyDamage _asbp_player 2.0 0 self)))

(event EventBeginPlay
  (bind _mesh (Variables|Character|GetMesh))
  (bind _returnvalue (Rendering|Material|CreateDynamicMaterialInstance _mesh 0 "/Game/Characters/GameChar/Xombi/Mats/M_Ch_1001.M_Ch_1001" "None" :!class /Script/Engine.PrimitiveComponent))
  (bind _returnvalue_2 (Rendering|Material|CreateDynamicMaterialInstance _mesh 1 "/Game/Characters/GameChar/Xombi/Mats/M_Ch_1002.M_Ch_1002" "None" :!class /Script/Engine.PrimitiveComponent))
  (bind _output_get (Variables|Default|SetDissolveMat1 _returnvalue))
  (bind _output_get_2 (Variables|Default|SetDissolveMat2 _returnvalue_2))
  (Rendering|Material|SetScalarParameterValue _output_get "Dissolve" 0.0 :!class /Script/Engine.MaterialInstanceDynamic)
  (bind _dissolve (Timeline|Timeline_0 ReverseFromEnd)
    (:Update
      (Rendering|Material|SetScalarParameterValue _output_get "Dissolve" _dissolve :!class /Script/Engine.MaterialInstanceDynamic))
    (:Finished
      (AI|AIMoveTo self "0, 0, 0" (Game|GetPlayerCharacter 0) 1e+02 false :!label _label
        (:then
          (Variables|/Script/Engine.CharacterMovementComponent|SetMaxWalkSpeed (Variables|Character|GetCharacterMovement) 5e+02))
        (:OnSuccess
          (Components|Animation|PlayAnimation (Variables|Character|GetMesh) "/Game/Characters/GameChar/Animations/Xombie/zombie_attack.zombie_attack" false)
          (Utilities|FlowControl|Delay 4.0)
          (if (not (<= (Variables|Default|GetXombiHP) 0.0))
            (Components|Animation|SetAnimationMode (Variables|Character|GetMesh) "AnimationBlueprint" true)
            (goto _label)))
        (:OnFail
          (Utilities|FlowControl|Delay 0.2)
          (goto _label))))))

(event Game|Damage|EventAnyDamage
  (params (Damage :type Float%20%28single-precision%29) (DamageType :type Damage%20Type%20Object%20Reference) (InstigatedBy :type Controller%20Object%20Reference) (DamageCauser :type Actor%20Object%20Reference))
  (bind _mesh (Variables|Character|GetMesh))
  (bind _output_get (Variables|Default|SetXombiHP (- (Variables|Default|GetXombiHP) Damage)))
  (if (< _output_get 1.0)
    (CallFunction|ZombieDead)
    (bind _returnvalue (Rendering|Material|CreateDynamicMaterialInstance _mesh 0 "/Game/Characters/GameChar/Xombi/Mats/M_Ch_1001.M_Ch_1001" "None" :!class /Script/Engine.PrimitiveComponent))
    (bind _returnvalue_2 (Rendering|Material|CreateDynamicMaterialInstance _mesh 1 "/Game/Characters/GameChar/Xombi/Mats/M_Ch_1002.M_Ch_1002" "None" :!class /Script/Engine.PrimitiveComponent))
    (bind _output_get_2 (Variables|Default|SetDissolveMat1 _returnvalue))
    (bind _output_get_3 (Variables|Default|SetDissolveMat2 _returnvalue_2))
    (Rendering|Material|SetScalarParameterValue _output_get_2 "Dissolve" 0.0 :!class /Script/Engine.MaterialInstanceDynamic)
    (bind _dissolve (Timeline|Timeline PlayFromStart)
      (:Update
        (Rendering|Material|SetScalarParameterValue _output_get_2 "Dissolve" _dissolve :!class /Script/Engine.MaterialInstanceDynamic)))
    (else
      (CallFunction|ZombieHit)
      (Components|Animation|SetAnimationMode (Variables|Character|GetMesh) "AnimationBlueprint" true)
      (AI|AIMoveTo self "0, 0, 0" (Game|GetPlayerCharacter 0) 1e+02 false :!label _label
        (:then
          (Variables|/Script/Engine.CharacterMovementComponent|SetMaxWalkSpeed (Variables|Character|GetCharacterMovement) 5e+02))
        (:OnSuccess
          (Components|Animation|PlayAnimation (Variables|Character|GetMesh) "/Game/Characters/GameChar/Animations/Xombie/zombie_attack.zombie_attack" false)
          (Utilities|FlowControl|Delay 4.0)
          (if (not (<= (Variables|Default|GetXombiHP) 0.0))
            (Components|Animation|SetAnimationMode (Variables|Character|GetMesh) "AnimationBlueprint" true)
            (goto _label)))
        (:OnFail
          (Utilities|FlowControl|Delay 0.2)
          (goto _label))))))

(fn ConstructionScript
  (|CallParentFunction))