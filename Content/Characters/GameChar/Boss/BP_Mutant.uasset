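; Boss mutant character that dissolves in on spawn, then chases the player with AIMoveTo and attacks in a loop.
; Above a health threshold it swipes with hand hitboxes; below it, it telegraphs an explosive AOE jump attack with a ground marker, also retriggered from Tick via Delay.
; Tick reports boss health and adjusts speed by health.
; Death dissolves the mesh before signalling the kill; winning plays a Macarena dance.
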(event OnComponentBeginOverlap(Right)
  (params (OverlappedComponent :type Primitive%20Component%20Object%20Reference) (OtherActor :type Actor%20Object%20Reference) (OtherComp :type Primitive%20Component%20Object%20Reference) (OtherBodyIndex :type Integer) (bFromSweep :type Boolean) (SweepResult :type Hit%20Result%20Structure%20%28by%20ref%29))
  (bind _self self)
  ;[1 1 1] attack damage
  (bind _asbp_player (Utilities|Casting|CastToBP_Player OtherActor))
  (bind _returnvalue (Game|Damage|ApplyDamage _asbp_player 1e+02 0 self))
  (if (<= (- (Variables|/Game/Characters/GameChar/Main/BP_Player.BP_Player_C|GetPlayerHP (stale OnComponentBeginOverlap(Left) _asbp_player)) (+ _returnvalue (stale OnComponentBeginOverlap(Left) _returnvalue))) 0.0)
    (CallFunction|MutantWin _self _self _self)))

(event OnComponentBeginOverlap(Left)
  (params (OverlappedComponent :type Primitive%20Component%20Object%20Reference) (OtherActor :type Actor%20Object%20Reference) (OtherComp :type Primitive%20Component%20Object%20Reference) (OtherBodyIndex :type Integer) (bFromSweep :type Boolean) (SweepResult :type Hit%20Result%20Structure%20%28by%20ref%29))
  (bind _self self)
  ;[1 1 1] attack damage
  (bind _asbp_player (Utilities|Casting|CastToBP_Player OtherActor))
  (bind _returnvalue (Game|Damage|ApplyDamage _asbp_player 1e+02 0 self))
  (if (<= (- (Variables|/Game/Characters/GameChar/Main/BP_Player.BP_Player_C|GetPlayerHP _asbp_player) (+ (stale OnComponentBeginOverlap(Right) _returnvalue) _returnvalue)) 0.0)
    (CallFunction|MutantWin _self _self _self)))

(event OnComponentBeginOverlap(AOE)
  (params (OverlappedComponent :type Primitive%20Component%20Object%20Reference) (OtherActor :type Actor%20Object%20Reference) (OtherComp :type Primitive%20Component%20Object%20Reference) (OtherBodyIndex :type Integer) (bFromSweep :type Boolean) (SweepResult :type Hit%20Result%20Structure%20%28by%20ref%29))
  ;[1 1 1] jump attack damage
  (bind _asbp_player (Utilities|Casting|CastToBP_Player OtherActor))
  (bind _returnvalue (Game|Damage|ApplyDamage _asbp_player 1e+03 0 self))
  (bind _output_get (Variables|Default|SetPlayerHP (- (Variables|Default|GetPlayerHP) _returnvalue))))

(event EventBeginPlay
  (bind _self self)
  (bind _self_2 self)
  (bind _cylinder (Variables|Default|GetCylinder))
  (bind _returnvalue (Transformation|GetWorldLocation _cylinder))
  (bind _returnvalue_2 (Rendering|Material|CreateDynamicMaterialInstance (Variables|Character|GetMesh) 0 "/Game/Characters/GameChar/Boss/Materials/mutant_M.mutant_M" "None" :!class /Script/Engine.PrimitiveComponent))
  (bind _output_get (Variables|Default|SetDissolve _returnvalue_2))
  (Rendering|Material|SetScalarParameterValue _output_get "Dissolve" 0.0 :!class /Script/Engine.MaterialInstanceDynamic)
  (bind _dissolve (Timeline|Timeline ReverseFromEnd)
    (:Update
      (Rendering|Material|SetScalarParameterValue _output_get "Dissolve" _dissolve :!class /Script/Engine.MaterialInstanceDynamic))
    (:Finished
      (Utilities|FlowControl|Delay 2.0)
      (AI|AIMoveTo self "0, 0, 0" (Pawn|GetControlledPawn (Game|GetPlayerController 0)) 3.5e+02 false :!label _label
        (:OnSuccess
          (if (< (Variables|Default|GetBossHP) 1.5e+03)
            (Rendering|Material|SetMaterial (Variables|Default|GetCylinder) 0 "/Game/Common/target_Mat.target_Mat")
            (Components|Animation|PlayAnimation (Variables|Character|GetMesh) "/Game/Characters/GameChar/Animations/Mutant/JUMP_ATTACK_FOOL.JUMP_ATTACK_FOOL" false)
            (Utilities|FlowControl|Delay 1.5)
            (CallFunction|TurnonHitboxAOE)
            (Effects|SpawnEmitteratLocation "/Game/StarterContent/Particles/P_Explosion.P_Explosion" _returnvalue "0, 0, 0" (Transformation|GetWorldScale _cylinder))
            (Audio|PlaySoundatLocation "/Game/StarterContent/Audio/Explosion01.Explosion01" _returnvalue "0, 0, 0" 1.0 1.0 0.0 0 0 0 0)
            (Utilities|FlowControl|Delay 0.5)
            (CallFunction|TurnOffHitboxAOE)
            (Rendering|Material|SetMaterial (Variables|Default|GetCylinder) 0 "/Game/Common/target_Mat_Inv.target_Mat_Inv")
            (Utilities|FlowControl|Delay 2.0)
            (if (< (stale OnComponentBeginOverlap(AOE) _output_get) 1.0)
              (CallFunction|MutantWin _self_2 _self_2 _self_2)
              (else
                (Components|Animation|SetAnimationMode (Variables|Character|GetMesh) "AnimationBlueprint" true)
                (goto _label)))
            (else
              (Components|Animation|PlayAnimation (Variables|Character|GetMesh) "/Game/Characters/GameChar/Animations/Mutant/mutant_swiping.mutant_swiping" false)
              (Audio|PlaySoundatLocation "/Game/Audio/bossattack.bossattack" "0, 0, 0" "0, 0, 0" 1.0 1.0 1.0 0 0 0 0)
              (Utilities|FlowControl|Delay 3.0)
              (if (< (Variables|Default|GetPlayerHP) 1.0)
                (CallFunction|MutantWin _self _self _self)
                (elif (not (<= (Variables|Default|GetBossHP) 0.0))
                  (Components|Animation|SetAnimationMode (Variables|Character|GetMesh) "AnimationBlueprint" true)
                  (goto _label))))))))))

(event Game|Damage|EventAnyDamage
  (params (Damage :type Float%20%28single-precision%29) (DamageType :type Damage%20Type%20Object%20Reference) (InstigatedBy :type Controller%20Object%20Reference) (DamageCauser :type Actor%20Object%20Reference))
  (bind _output_get (Variables|Default|SetBossHP (- (Variables|Default|GetBossHP) Damage)))
  (Audio|PlaySoundatLocation "/Game/Audio/bosshurt.bosshurt" (Transformation|GetActorLocation) "0, 0, 0" 1.0 1.0 1.0 0 0 0 0)
  (if (< _output_get 1.0)
    (CallFunction|MutantDead)
    (bind _returnvalue (Rendering|Material|CreateDynamicMaterialInstance (Variables|Character|GetMesh) 0 "/Game/Characters/GameChar/Boss/Materials/mutant_M.mutant_M" "None" :!class /Script/Engine.PrimitiveComponent))
    (bind _output_get_2 (Variables|Default|SetDissolve _returnvalue))
    (Rendering|Material|SetScalarParameterValue _output_get_2 "Dissolve" 0.0 :!class /Script/Engine.MaterialInstanceDynamic)
    (bind _dissolve (Timeline|DissolveFX PlayFromStart)
      (:Update
        (Rendering|Material|SetScalarParameterValue _output_get_2 "Dissolve" _dissolve :!class /Script/Engine.MaterialInstanceDynamic))
      (:Finished
        (Default|CallBossKilled)))))

(event EventTick
  (params (DeltaSeconds :type Float%20%28single-precision%29))
  (bind _self self)
  (bind _self_2 self)
  (bind _aoe (Variables|Default|GetAOE))
  (bind _cylinder (Variables|Default|GetCylinder))
  (bind _charactermovement (Variables|Character|GetCharacterMovement))
  (bind _returnvalue (Transformation|GetWorldLocation _cylinder))
  (bind _returnvalue_2 (Transformation|GetWorldLocation _aoe))
  (Default|CallBossHealth (Variables|Default|GetBossHP))
  (if (< (Variables|Default|GetBossHP) 1.5e+03)
    (Variables|/Script/Engine.CharacterMovementComponent|SetMaxWalkSpeed _charactermovement 6e+02)
    (if (< (Variables|Default|GetBossHP) 1e+02)
      (Variables|/Script/Engine.CharacterMovementComponent|SetMaxWalkSpeed _charactermovement 8e+02))
    (Transformation|SetWorldLocation (Variables|Default|GetCylinder) (Math|Vector|MakeVector (.x _returnvalue_2) (.y _returnvalue_2) 15.0) false false)
    (Transformation|SetWorldRotation (Variables|Default|GetCylinder) "0, 0, 0" false false)
    (if (not (< (Variables|Default|GetPlayerHP) 0.0))
      (Utilities|FlowControl|Delay 15.0)
      (Rendering|Material|SetMaterial (Variables|Default|GetCylinder) 0 "/Game/Common/target_Mat.target_Mat" :!label _label)
      (Components|Animation|PlayAnimation (Variables|Character|GetMesh) "/Game/Characters/GameChar/Animations/Mutant/JUMP_ATTACK_FOOL.JUMP_ATTACK_FOOL" false)
      (Utilities|FlowControl|Delay 1.5)
      (CallFunction|TurnonHitboxAOE)
      (Effects|SpawnEmitteratLocation "/Game/StarterContent/Particles/P_Explosion.P_Explosion" _returnvalue "0, 0, 0" (Transformation|GetWorldScale _cylinder))
      (Audio|PlaySoundatLocation "/Game/StarterContent/Audio/Explosion01.Explosion01" _returnvalue "0, 0, 0" 1.0 1.0 0.0 0 0 0 0)
      (Utilities|FlowControl|Delay 0.5)
      (CallFunction|TurnOffHitboxAOE)
      (Rendering|Material|SetMaterial (Variables|Default|GetCylinder) 0 "/Game/Common/target_Mat_Inv.target_Mat_Inv")
      (Utilities|FlowControl|Delay 2.0)
      (if (< (stale OnComponentBeginOverlap(AOE) _output_get) 1.0)
        (CallFunction|MutantWin _self_2 _self_2 _self_2)
        (else
          (Components|Animation|SetAnimationMode (Variables|Character|GetMesh) "AnimationBlueprint" true)
          (AI|AIMoveTo self "0, 0, 0" (Pawn|GetControlledPawn (Game|GetPlayerController 0)) 3.5e+02 false :!label _label_2
            (:OnSuccess
              (if (< (Variables|Default|GetBossHP) 1.5e+03)
                (goto _label)
                (else
                  (Components|Animation|PlayAnimation (Variables|Character|GetMesh) "/Game/Characters/GameChar/Animations/Mutant/mutant_swiping.mutant_swiping" false)
                  (Audio|PlaySoundatLocation "/Game/Audio/bossattack.bossattack" "0, 0, 0" "0, 0, 0" 1.0 1.0 1.0 0 0 0 0)
                  (Utilities|FlowControl|Delay 3.0)
                  (if (< (Variables|Default|GetPlayerHP) 1.0)
                    (CallFunction|MutantWin _self _self _self)
                    (elif (not (<= (Variables|Default|GetBossHP) 0.0))
                      (Components|Animation|SetAnimationMode (Variables|Character|GetMesh) "AnimationBlueprint" true)
                      (goto _label_2))))))))))
    (else
      (Variables|/Script/Engine.CharacterMovementComponent|SetMaxWalkSpeed _charactermovement 7e+02))))

(fn ConstructionScript)

(fn MutantDead
  (bind _charactermovement (Variables|Character|GetCharacterMovement))
  (Pawn|Components|CharacterMovement|DisableMovement _charactermovement)
  (Class|NavMovementComponent|StopActiveMovement _charactermovement)
  (Components|Movement|StopMovementImmediately _charactermovement)
  (Pawn|Components|CharacterMovement|SetMovementMode _charactermovement "MOVE_Walking" 0)
  (Components|Animation|PlayAnimation (Variables|Character|GetMesh) "/Game/Characters/GameChar/Animations/Xombie/Zombie_Death.Zombie_Death" false)
  (Actor|SetLifeSpan 8.0)
  (Collision|SetCollisionEnabled (Variables|Default|GetLeft) "NoCollision")
  (Components|DestroyComponent (Variables|Default|GetCylinder))
  (Audio|PlaySoundatLocation "/Game/Audio/bossdeath.bossdeath" (Transformation|GetActorLocation) "0, 0, 0" 1.0 1.0 0.0 0 0 0 0))

(fn MutantWin
  (params (self2 :type Character%20Object%20Reference) (self3 :type Character%20Object%20Reference) (self4 :type Character%20Object%20Reference))
  (bind _charactermovement (Variables|Character|GetCharacterMovement))
  (Pawn|Components|CharacterMovement|DisableMovement _charactermovement)
  (Class|NavMovementComponent|StopActiveMovement _charactermovement)
  (Components|Movement|StopMovementImmediately _charactermovement)
  (Pawn|Components|CharacterMovement|SetMovementMode _charactermovement "MOVE_Walking" 0)
  (Collision|SetCollisionEnabled (Variables|Default|GetLeft) "NoCollision")
  (Components|Animation|PlayAnimation (Variables|Character|GetMesh) "/Game/Characters/GameChar/Animations/Mutant/Macarena_Dance.Macarena_Dance" true))

(fn TurnonHitboxAOE
  (bind _aoe (Variables|Default|GetAOE))
  (Collision|SetCollisionEnabled _aoe "QueryAndPhysics")
  (Collision|SetCollisionProfileName _aoe "BlockAllDynamic" true :!class /Script/Engine.PrimitiveComponent)
  (Collision|SetCollisionObjectType _aoe "ECC_WorldDynamic")
  (Collision|SetCollisionResponsetoAllChannels _aoe "ECR_Overlap"))

(fn TurnOffHitboxAOE
  (bind _aoe (Variables|Default|GetAOE))
  (Collision|SetCollisionEnabled _aoe "NoCollision")
  (Collision|SetCollisionProfileName _aoe "NoCollision" true :!class /Script/Engine.PrimitiveComponent)
  (Collision|SetCollisionObjectType _aoe "ECC_WorldStatic")
  (Collision|SetCollisionResponsetoAllChannels _aoe "ECR_Ignore"))