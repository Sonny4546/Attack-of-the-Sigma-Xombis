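; BP_Bullet is a projectile actor that damages actors it overlaps and pushes physics objects it hits.
; Capsule begin-overlap applies fixed damage to the other actor and spawns a blood splatter effect at the bullet's location.
; A hit adds a velocity-scaled impulse to simulating components, then destroys the bullet.
; Capsule end-overlap also destroys it, so damage and destruction occur on separate overlap events.
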(event OnComponentBeginOverlap(Capsule)
  (params (OverlappedComponent :type Primitive%20Component%20Object%20Reference) (OtherActor :type Actor%20Object%20Reference) (OtherComp :type Primitive%20Component%20Object%20Reference) (OtherBodyIndex :type Integer) (bFromSweep :type Boolean) (SweepResult :type Hit%20Result%20Structure%20%28by%20ref%29))
  (Game|Damage|ApplyDamage OtherActor 1e+01 0 self)
  (Niagara|SpawnSystematLocation "/Game/Common/Particles/bloodsplatter.bloodsplatter" (Transformation|GetActorLocation)))

(event OnComponentEndOverlap(Capsule)
  (params (OverlappedComponent :type Primitive%20Component%20Object%20Reference) (OtherActor :type Actor%20Object%20Reference) (OtherComp :type Primitive%20Component%20Object%20Reference) (OtherBodyIndex :type Integer))
  (Actor|DestroyActor))

(event Collision|EventHit
  (params (MyComp :type Primitive%20Component%20Object%20Reference) (Other :type Actor%20Object%20Reference) (OtherComp :type Primitive%20Component%20Object%20Reference) (bSelfMoved :type Boolean) (HitLocation :type Vector :default "0, 0, 0") (HitNormal :type Vector :default "0, 0, 0") (NormalImpulse :type Vector :default "0, 0, 0") (Hit :type Hit%20Result%20Structure%20%28by%20ref%29))
  (if (Physics|IsSimulatingPhysics OtherComp "None")
    (Physics|AddImpulseatLocation OtherComp (* (Transformation|GetVelocity) 1e+01) (Transformation|GetActorLocation) "None"))
  (Actor|DestroyActor))

(fn ConstructionScript)